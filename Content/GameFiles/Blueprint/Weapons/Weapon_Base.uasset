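; Base weapon Blueprint for a hitscan gun used by the player character, with ammo, recoil and scope view setup.
; FireEvent spends magazine ammo, traces from the camera with spread during free fire, ejects a temporary shell and applies random recoil.
; It loops for burst fire or briefly locks firing and exits the scope, while FireEffects selects impacts and decals by physical surface.
; ReloadEvent refills from bag ammo and updates the player's HUD.
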(event Custom|FireEvent
  (bind _returnvalue (Game|GetPlayerCameraManager 0))
  (bind _weaponrange (Variables|Default|GetWeaponRange))
  (bind _playerref (Variables|Default|GetPlayerRef))
  (bind _spreadrange (Variables|Default|GetSpreadRange))
  (bind _returnvalue_2 (Camera|GetCameraLocation _returnvalue))
  (bind _returnvalue_3 (Transformation|GetActorForwardVector _returnvalue))
  (bind _returnvalue_4 (* _spreadrange -1.0))
  (bind _returnvalue_5 (* _returnvalue_3 _weaponrange))
  (bind _returnvalue_6 (+ _returnvalue_5 _returnvalue_2))
  (bind (_x _y _z) (Math|Vector|BreakVector _returnvalue_6))
  ;[1 1 1] Fire Event
  (bind _result (CallFunction|AmmoCalculate (Variables|Default|GetFireAmmoCount) :!label _label))
  (if _result
    (bind (_outhit _returnvalue_7) (Collision|LineTraceByChannel _returnvalue_2 (select (Variables|/Game/AdvancedLocomotionV4/Blueprints/CharacterLogic/PlayerCharacter.PlayerCharacter_C|GetFreeFire (Variables|Default|GetPlayerRef)) (Math|Vector|MakeVector (+ _x (Math|Random|RandomFloatinRange _returnvalue_4 _spreadrange)) (+ _y (Math|Random|RandomFloatinRange _returnvalue_4 _spreadrange)) (+ _z (Math|Random|RandomFloatinRange _returnvalue_4 _spreadrange))) _returnvalue_6) "TraceTypeQuery1" false 0 "None"))
    (CallFunction|FireEffects _outhit _returnvalue_7)
    (bind _returnvalue_8 (Game|SpawnActorfromClass (Variables|Default|GetShellEject) (Transformation|GetSocketTransform (Variables|Default|GetGunMesh) "AmmoEject" "RTS_World") "Undefined" 0 0))
    (Utilities|FlowControl|Sequence
      (:then_0
        (CallFunction|WeaponRecoil)
        (if (Variables|Default|GetBurstFire)
          (if (Variables|Default|GetBurstEnabled)
            (if (Variables|/Game/AdvancedLocomotionV4/Blueprints/CharacterLogic/PlayerCharacter.PlayerCharacter_C|GetIsFiring (Variables|Default|GetPlayerRef))
              (Utilities|FlowControl|Delay (Variables|Default|GetFireRecoverTime))
              (goto _label)))
          (else
            (Variables|/Game/AdvancedLocomotionV4/Blueprints/CharacterLogic/PlayerCharacter.PlayerCharacter_C|SetCanFire _playerref false)
            (if (Widget|IsVisible (Variables|/Game/AdvancedLocomotionV4/Blueprints/CharacterLogic/PlayerCharacter.PlayerCharacter_C|GetScopeRef _playerref))
              (Default|ScopeExit _playerref))
            (Utilities|FlowControl|Delay (Variables|Default|GetFireRecoverTime))
            (Variables|/Game/AdvancedLocomotionV4/Blueprints/CharacterLogic/PlayerCharacter.PlayerCharacter_C|SetCanFire _playerref true))))
      (:then_1
        (Utilities|FlowControl|Delay 1.0)
        (Utilities|IsValid _returnvalue_8
          (:Is%20Valid
            (Actor|DestroyActor _returnvalue_8)))))))

(event Custom|WeaponRecoil
  (bind _recoilrange (Variables|Default|GetRecoilRange))
  (bind _returnvalue (/ _recoilrange 2.0))
  ;[1 1 1] Weapon Recoil
  (Pawn|Input|AddControllerPitchInput (Variables|Default|GetPlayerRef) (Math|Random|RandomFloatinRange -0.5 (* -1 (Variables|Default|GetRecoilRange))))
  (Pawn|Input|AddControllerYawInput (Variables|Default|GetPlayerRef) (Math|Random|RandomFloatinRange (* -1 _returnvalue) _returnvalue)))

(event Custom|Reload%20Event
  ;[1 1 1] Reload Event
  (if (> (Variables|Default|GetCurrentBagAmmo) 0)
    (if (== (Variables|Default|GetCurrentMagAmmo) 0)
      (if (>= (Variables|Default|GetCurrentBagAmmo) (Variables|Default|GetMagCapacity))
        (Variables|Default|SetCurrentMagAmmo (Variables|Default|GetMagCapacity))
        (Variables|Default|SetCurrentBagAmmo (- (Variables|Default|GetCurrentBagAmmo) (Variables|Default|GetMagCapacity)))
        (else
          (Variables|Default|SetCurrentMagAmmo (Variables|Default|GetCurrentBagAmmo))
          (Variables|Default|SetCurrentBagAmmo 0)))
      (elif (>= (Variables|Default|GetCurrentBagAmmo) (Variables|Default|GetMagCapacity))
        (Variables|Default|SetCurrentBagAmmo (- (Variables|Default|GetCurrentBagAmmo) (- (Variables|Default|GetMagCapacity) (Variables|Default|GetCurrentMagAmmo))))
        (Variables|Default|SetCurrentMagAmmo (Variables|Default|GetMagCapacity))
        (elif (> (- (Variables|Default|GetMagCapacity) (Variables|Default|GetCurrentMagAmmo)) (Variables|Default|GetCurrentBagAmmo))
          (Variables|Default|SetCurrentMagAmmo (Variables|Default|GetMagCapacity))
          (Variables|Default|SetCurrentBagAmmo (- (Variables|Default|GetCurrentBagAmmo) (- (Variables|Default|GetMagCapacity) (Variables|Default|GetCurrentMagAmmo))))
          (else
            (Variables|Default|SetCurrentMagAmmo (+ (Variables|Default|GetCurrentMagAmmo) (Variables|Default|GetCurrentBagAmmo)))
            (Variables|Default|SetCurrentBagAmmo 0)))))
    (Default|UpdateWeaponHud (Variables|Default|GetPlayerRef) 0 0 (Variables|Default|GetCurrentMagAmmo) 0 "NewEnumerator2")
    (Default|UpdateWeaponHud (Variables|Default|GetPlayerRef) 0 0 0 (Variables|Default|GetCurrentBagAmmo) "NewEnumerator3")))

(event Custom|FireEffects
  (params (HitResult :type Hit%20Result%20Structure) (ReturnValue :type Boolean))
  (bind (_bblockinghit _binitialoverlap _time _distance _location _impactpoint _normal _impactnormal _physmat _hitactor _hitcomponent) (Collision|BreakHitResult HitResult))
  (bind _decalsize (Variables|Default|GetDecalSize))
  (bind _surfacetype (Variables|/Script/PhysicsCore.PhysicalMaterial|GetSurfaceType _physmat))
  ;[1 1 1] Fire Effects Custom Event
  (Components|Animation|PlayAnimation (Variables|Default|GetGunMesh) (Variables|Default|GetMuzzleFlashEffects) false)
  (if ReturnValue
    (Effects|SpawnEmitteratLocation (Utilities|Select :Index _surfacetype :SurfaceType_Default (Variables|Default|GetDefaultEmitter) :SurfaceType1 (Variables|Default|GetConcreteEmitter) :SurfaceType2 (Variables|Default|GetWoodEmitter) :SurfaceType3 (Variables|Default|GetFleshEmitter)) _impactpoint)
    (Class|GameplayStatics|SpawnDecalAttached (Utilities|Select :Index _surfacetype :SurfaceType_Default "/Game/GameFiles/Blueprint/Weapons/ImpactEffects/Materials/BulletHoleDefault_Mat.BulletHoleDefault_Mat" :SurfaceType1 "/Game/GameFiles/Blueprint/Weapons/ImpactEffects/Materials/BulletHoleConcrete_Mat.BulletHoleConcrete_Mat" :SurfaceType2 "/Game/GameFiles/Blueprint/Weapons/ImpactEffects/Materials/BulletHoleWood_Mat.BulletHoleWood_Mat" :SurfaceType3 0) (Math|Vector|MakeVector _decalsize _decalsize _decalsize) _hitcomponent "None" _impactpoint (Math|Conversions|RotationFromXVector _normal) "KeepWorldPosition" 1e+01)))

(event EventBeginPlay
  ;[1 1 1] Begin Play
  (bind _asplayer_character (Utilities|Casting|CastToPlayerCharacter (Game|GetPlayerCharacter 0)))
  (Variables|Default|SetPlayerRef _asplayer_character)
  (Camera|SetFieldOfView (Variables|Default|GetADS) (Variables|Default|GetMaxScopeRange)))

(fn ConstructionScript)

(fn AmmoCalculate
  (params (AmmoCount :type Integer))
  (if (== (Variables|Default|GetCurrentMagAmmo) 0)
    (Default|UpdateWeaponHud (Variables|Default|GetPlayerRef) 0 0 (Variables|Default|GetCurrentMagAmmo) 0 "NewEnumerator2")
    (return false)
    (else
      (bind _output_get (Variables|Default|SetCurrentMagAmmo (- (Variables|Default|GetCurrentMagAmmo) AmmoCount)))
      (Default|UpdateWeaponHud (Variables|Default|GetPlayerRef) 0 0 _output_get 0 "NewEnumerator2")
      (return true))))