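; Base weapon pickup actor that gives the player a weapon with preset magazine and bag ammo on interaction.
; Overlapping its collision binds PickUp to the character's Interact event and shows that character's pickup HUD; leaving reverses both.
; PickUp calls SpawnWeapon on the player 0 character cached at BeginPlay, not the overlapping one, and destroys the pickup if that succeeds.
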(event OnComponentBeginOverlap(PickCollision)
  (params (OverlappedComponent :type Primitive%20Component%20Object%20Reference) (OtherActor :type Actor%20Object%20Reference) (OtherComp :type Primitive%20Component%20Object%20Reference) (OtherBodyIndex :type Integer) (bFromSweep :type Boolean) (SweepResult :type Hit%20Result%20Structure%20%28by%20ref%29))
  (bind _asplayer_character (Utilities|Casting|CastToPlayerCharacter OtherActor))
  (EventDispatchers|BindEventtoInteract _asplayer_character (delegate Custom|PickUp))
  (if (not (UserInterface|Viewport|IsinViewport (Variables|/Game/AdvancedLocomotionV4/Blueprints/CharacterLogic/PlayerCharacter.PlayerCharacter_C|GetWeaponPickHUD_Ref _asplayer_character)))
    (UserInterface|Viewport|AddtoViewport (Variables|/Game/AdvancedLocomotionV4/Blueprints/CharacterLogic/PlayerCharacter.PlayerCharacter_C|GetWeaponPickHUD_Ref _asplayer_character) 0)))

(event OnComponentEndOverlap(PickCollision)
  (params (OverlappedComponent :type Primitive%20Component%20Object%20Reference) (OtherActor :type Actor%20Object%20Reference) (OtherComp :type Primitive%20Component%20Object%20Reference) (OtherBodyIndex :type Integer))
  (bind _asplayer_character (Utilities|Casting|CastToPlayerCharacter OtherActor))
  (EventDispatchers|UnbindEventfromInteract _asplayer_character (delegate Custom|PickUp))
  (Widget|RemovefromParent (Variables|/Game/AdvancedLocomotionV4/Blueprints/CharacterLogic/PlayerCharacter.PlayerCharacter_C|GetWeaponPickHUD_Ref _asplayer_character)))

(event Custom|PickUp
  (bind _successful (Default|SpawnWeapon (Variables|Reference|GetPlayerRef) (Variables|Default|GetWeapon) (Variables|Default|GetWeaponSocket) (Variables|Default|GetMagAmmo) (Variables|Default|GetBagAmmo)))
  (if _successful
    (Actor|DestroyActor)))

(event EventBeginPlay
  ;[1 1 1] Begin Play
  (bind _asplayer_character (Utilities|Casting|CastToPlayerCharacter (Game|Player|GetPlayerPawn 0)))
  (Variables|Reference|SetPlayerRef _asplayer_character))

(fn ConstructionScript)